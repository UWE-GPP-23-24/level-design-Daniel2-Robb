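; Turret AI variant that fires BP_SimpleProjectileFaster projectiles at its target.
; Its attacking-state tick checks whether it can attack, then turns toward the target and runs its own FireAtTargetFaster function.
; That function accumulates delta time in a timer and, on reaching FireRate, spawns a projectile at the ProjectileSpawn transform with the turret as instigator, then resets the timer.
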(event Custom|CustomEvent
  (params (DeltaTime :type Float%20%28double-precision%29))
  ;[0.4491 0.8591 1] Attacking State - Tick
  (if (CallFunction|IsAbletoAttack)
    (Utilities|FlowControl|Sequence
      (:then_0
        (CallFunction|LookatTarget))
      (:then_1
        (CallFunction|FireatTargetFaster DeltaTime)))))

(event EventBeginPlay
  (|CallParentFunction) ; This node is disabled and will not be called.\nDrag off pins to build functionality.
)

(event Collision|EventActorBeginOverlap
  (params (OtherActor :type Actor%20Object%20Reference)))

(event EventTick
  (params (DeltaSeconds :type Float%20%28single-precision%29))
  (|CallParentFunction DeltaSeconds) ; This node is disabled and will not be called.\nDrag off pins to build functionality.
)

(fn ConstructionScript
  (|CallParentFunction))

(fn FireatTargetFaster
  (params (DeltaTime :type Float%20%28double-precision%29))
  (bind _projectilespawn (Variables|Default|GetProjectileSpawn))
  (bind _returnvalue (Transformation|GetWorldTransform _projectilespawn))
  (bind _output_get (Variables|Default|SetFireTimer (+ (Variables|Default|GetFireTimer) DeltaTime)))
  (if (>= _output_get (Variables|Default|GetFireRate))
    (Game|SpawnActorfromClass "/Game/GPP/Blueprints/Obstacles/BP_SimpleProjectileFaster.BP_SimpleProjectileFaster_C" (Math|Transform|MakeTransform (.location _returnvalue) (.rotation _returnvalue) "1.000000,1.000000,1.000000") "AlwaysSpawn" "MultiplyWithRoot" 0 self)
    (Variables|Default|SetFireTimer 0.0)))
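; Moving platform variant that stays idle until triggered, responding only to the first trigger.
; The Triggered event sets a flag that Tick consumes to call MovePlatform.
; MovePlatform snaps the platform to StartPoint, targets EndPoint, waits, then calls MoveToTarget and sets the timeline play rate from MoveSpeed.
; With one stop or fewer, it uses a fixed delay and forces Stops to two.
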(event Custom|Triggered
  (Development|PrintString "Trigger Hit")
  (if (Variables|Default|GetFirstTrigger)
    (Variables|Default|SetTriggered? true)
    (Variables|Default|SetFirstTrigger false)))

(event Custom|MovePlatform
  ;[0.4491 0.8591 1] Initialise to the start location
  (Transformation|SetWorldLocation (Variables|Default|GetPlatform) (Transformation|GetWorldLocation (Variables|Default|GetStartPoint)) false true)
  ;[0.4491 0.8591 1] Set target and current points
  (Variables|Default|SetTargetPoint (Variables|Default|GetEndPoint))
  (Variables|Default|SetCurrentPoint (Variables|Default|GetStartPoint))
  (if (> (Variables|Default|GetStops) 1)
    (Utilities|FlowControl|Delay (Variables|Default|GetDelayBetweenPoints))
    (else
      (Utilities|FlowControl|Delay 0.75)
      (Variables|Default|SetStops 2)))
  (CallFunction|MovetoTarget)
  (Components|Timeline|SetPlayRate (Variables|Default|GetMoveTimeline) (Variables|Default|GetMoveSpeed)))

(event EventTick
  (params (DeltaSeconds :type Float%20%28single-precision%29))
  (if (Variables|Default|GetTriggered?)
    (Variables|Default|SetTriggered? false)
    (CallFunction|MovePlatform)))

(event EventBeginPlay
  (Variables|Default|SetTriggered? false)
  (Variables|Default|SetFirstTrigger true))

(fn ConstructionScript
  (|CallParentFunction))